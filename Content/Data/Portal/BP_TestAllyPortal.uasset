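; BP_TestAllyPortal is a test portal actor that spawns an allied character when the player walks into it.
; A sphere overlap filtered to BP_MainPlayer spawns a BP_Ally at the portal's scene component location.
; It then initializes that ally with hardcoded stats, skills, modular mesh parts, a staff weapon and an anim class, and assigns it a tag.
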(event OnComponentBeginOverlap(Sphere)
  (params (OverlappedComponent :type Primitive%20Component%20Object%20Reference) (OtherActor :type Actor%20Object%20Reference) (OtherComp :type Primitive%20Component%20Object%20Reference) (OtherBodyIndex :type Integer) (bFromSweep :type Boolean) (SweepResult :type Hit%20Result%20Structure%20%28by%20ref%29))
  (bind _asbp_main_player (Utilities|Casting|CastToBP_MainPlayer OtherActor))
  (Utilities|IsValid _asbp_main_player
    (:Is%20Valid
      (bind _returnvalue (Game|SpawnActorfromClass "/Game/ThirdPerson/Blueprints/BP_Ally.BP_Ally_C" (Math|Transform|MakeTransform (Transformation|GetWorldLocation (Variables|Default|GetScene)) "0, 0, 0" "1.000000,1.000000,1.000000") "Undefined" "MultiplyWithRoot" 0 0))
      (Class|GameCharacterBase|InitCharInfo _returnvalue "Ally" (Variables|Default|Getm_Stat) (Variables|Default|Getm_Skill) 1 "/Game/Characters/CR/LQ/Modular_001_Kingdom/Parts/Chest/SKM_ChestAM_020_8.SKM_ChestAM_020_8" (Utilities|Array|MakeArray "/Game/Characters/CR/LQ/Modular_001_Kingdom/Parts/Body/SKM_Head_001_1.SKM_Head_001_1" "/Game/Characters/CR/LQ/Modular_001_Kingdom/Parts/Hair/SKM_Hair_026_6.SKM_Hair_026_6" "/Game/Characters/CR/LQ/Modular_001_Kingdom/Parts/Face/SKM_Face_013_6.SKM_Face_013_6" "/Game/Characters/CR/LQ/Modular_001_Kingdom/Parts/Shoulder/SKM_ShoulderAM_003_4.SKM_ShoulderAM_003_4" "/Game/Characters/CR/LQ/Modular_001_Kingdom/Parts/Hand/SKM_HandAM_003_4.SKM_HandAM_003_4" "/Game/Characters/CR/LQ/Modular_001_Kingdom/Parts/Leg/SKM_LegAM_008_4.SKM_LegAM_008_4" "/Game/Characters/CR/LQ/Modular_001_Kingdom/Parts/Foot/SKM_FootAM_001_4.SKM_FootAM_001_4") "/Game/Characters/CR/LQ/Modular_001_Kingdom/Weapon/Staff/SM_Staff_002_4.SM_Staff_002_4" 0 "/Game/AnimBlueprint/Ally/ABP_Ally.ABP_Ally_C" "1.000000,1.000000,1.000000")
      (Variables|/Script/Engine.Actor|SetTags _returnvalue (Utilities|Array|MakeArray (Variables|Default|GetTag))))))

(fn ConstructionScript)